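; BP_CeilingLight is a configurable ceiling light actor with a point light that turns on when something overlaps its trigger.
; The construction script applies the brightness, color, source radius and on/off variables to PointLight1, and BeginPlay repeats this so data-only Blueprint versions update at runtime.
; Ending the overlap turns the light off unless PermanentLightOn is set.
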(event `self.ReceiveBeginPlay`
  (bind _pointlight1 (`self.PointLight1`))
  ;[1 1 1] Adding this here so the Data Only Blueprint version will update at runtime
  (`LightComponent.SetIntensity` _pointlight1 (`self.Brightness`))
  (`LightComponent.SetLightColor` _pointlight1 (`self.Color`) true)
  (`PointLightComponent.SetSourceRadius` _pointlight1 (`self.Source Radius`))
  (`SceneComponent.SetVisibility` (`self.PointLight1`) (`self.LightOn?`) false))

(event `self.Trigger.OnComponentBeginOverlap`
  (params (OverlappedComponent :type "PrimitiveComponent Object Reference") (OtherActor :type "Actor Object Reference") (OtherComp :type "PrimitiveComponent Object Reference") (OtherBodyIndex :type Integer) (bFromSweep :type Boolean) (SweepResult :type "HitResult Structure (by ref)"))
  (`SceneComponent.SetVisibility` (`self.PointLight1`) true false))

(event `self.Trigger.OnComponentEndOverlap`
  (params (OverlappedComponent :type "PrimitiveComponent Object Reference") (OtherActor :type "Actor Object Reference") (OtherComp :type "PrimitiveComponent Object Reference") (OtherBodyIndex :type Integer))
  (if (not (`self.PermanentLightOn?`))
    (`SceneComponent.SetVisibility` (`self.PointLight1`) false false)))

(fn `UserConstructionScript`
  (bind _pointlight1 (`self.PointLight1`))
  (`LightComponent.SetIntensity` _pointlight1 (`self.Brightness`))
  (`LightComponent.SetLightColor` _pointlight1 (`self.Color`) true)
  (`PointLightComponent.SetSourceRadius` _pointlight1 (`self.Source Radius`))
  (`SceneComponent.SetVisibility` _pointlight1 (`self.LightOn?`) false))